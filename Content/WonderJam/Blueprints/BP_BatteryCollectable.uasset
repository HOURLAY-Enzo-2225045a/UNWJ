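; BP_BatteryCollectable is a battery pickup that the first-person character collects to feed its flashlight.
; On overlap it registers itself as the character's interact object and shows an interaction prompt through the HUD's UI reference; leaving the overlap clears both.
; Its Interact event adds a battery to the character's FlashlightComponent and destroys the actor.
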(event EventBeginPlay)

(event Collision|EventActorBeginOverlap
  (params (OtherActor :type Actor%20Object%20Reference))
  (Development|PrintText "Begin Overlap")
  (bind _asbp_first_person_character (Utilities|Casting|CastToBP_FirstPersonCharacter OtherActor)
    (:then
      (bind _output_get (Variables|Default|SetCharacter _asbp_first_person_character))
      (Variables|/Game/FirstPerson/Blueprints/BP_FirstPersonCharacter.BP_FirstPersonCharacter_C|SetInteractObj _output_get self)
      (bind _asbp_hud (Utilities|Casting|CastToBP_HUD (HUD|GetHUD (Game|GetPlayerController 0))))
      (Variables|/Script/UMG.TextBlock|SetText (Variables|/Game/WonderJam/UI/UI_HUDDisplay.UI_HUDDisplay_C|GetInteractionText (Variables|/Game/WonderJam/Blueprints/BP_HUD.BP_HUD_C|GetUIReference _asbp_hud)) "Press [E] to interact"))
    (:CastFailed
      (Development|PrintText "Cast Failed"))))

(event Collision|EventActorEndOverlap
  (params (OtherActor :type Actor%20Object%20Reference))
  (bind _asbp_first_person_character (Utilities|Casting|CastToBP_FirstPersonCharacter OtherActor))
  (bind _output_get (Variables|Default|SetCharacter _asbp_first_person_character))
  (Variables|/Game/FirstPerson/Blueprints/BP_FirstPersonCharacter.BP_FirstPersonCharacter_C|SetInteractObj _output_get 0)
  (bind _asbp_hud (Utilities|Casting|CastToBP_HUD (HUD|GetHUD (Game|GetPlayerController 0))))
  (Variables|/Script/UMG.TextBlock|SetText (Variables|/Game/WonderJam/UI/UI_HUDDisplay.UI_HUDDisplay_C|GetInteractionText (Variables|/Game/WonderJam/Blueprints/BP_HUD.BP_HUD_C|GetUIReference _asbp_hud)) ""))

(event EventOnFeedback)

(event EventInteract
  (params (Controller :type Player%20Controller%20Object%20Reference))
  (Default|AddBattery (Variables|/Game/FirstPerson/Blueprints/BP_FirstPersonCharacter.BP_FirstPersonCharacter_C|GetFlashlightComponent (Variables|Default|GetCharacter)))
  (Actor|DestroyActor))

(fn ConstructionScript)