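; Actor component that manages a flashlight's on/off state and battery.
; While on and unpaused, Tick uses a Delay to drain the battery in half-second steps, switching the light off when nearly empty.
; OnOff only turns on with charge left, AddBattery adds clamped charge, and TogglePause suspends draining.
; State changes fire an OnFlashlightStatusChanged dispatcher, and debug prints report values.
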(event EventTick
  (params (DeltaSeconds :type Float%20%28single-precision%29))
  (if (not (Variables|Default|GetIsPaused))
    ;[1 1 1] Depleting the battery
    (if (Variables|Default|GetFlashlightStatus)
      (Utilities|FlowControl|Delay 0.5)
      (bind _output_get (Variables|Default|SetCurrentBattery (- (Variables|Default|GetCurrentBattery) 5.0)))
      (Development|PrintString (Utilities|String|ToString(Float) _output_get) true true "(R=1.000000,G=0.823529,B=0.000000,A=1.000000)")
      ;[1 1 1] Turn Off when no battery
      (if (< _output_get 1.0)
        (if (Variables|Default|GetFlashlightStatus)
          (bind _output_get_2 (Variables|Default|SetFlashlightStatus false))
          (Default|CallOnFlashlightStatusChanged)
          (Development|PrintString (Utilities|String|ToString(Boolean) _output_get_2) true true "(R=1.000000,G=0.823529,B=0.000000,A=1.000000)"))))))

(fn On/Off
  (if (Variables|Default|GetFlashlightStatus)
    (bind _output_get (Variables|Default|SetFlashlightStatus (not (Variables|Default|GetFlashlightStatus)) :!label _label))
    (Development|PrintString (Utilities|String|ToString(Boolean) _output_get))
    (Default|CallOnFlashlightStatusChanged)
    (elif (> (Variables|Default|GetCurrentBattery) 0.0)
      (goto _label))))

(fn AddBattery
  (bind _output_get (Variables|Default|SetCurrentBattery (Math|Float|Clamp(Float) (+ (Variables|Default|GetCurrentBattery) 35.0) 0.0 (Variables|Default|GetMaxBattery))))
  (Development|PrintString (Utilities|String|ToString(Float) _output_get)))

(fn TogglePause
  (bind _output_get (Variables|Default|SetIsPaused (not (Variables|Default|GetIsPaused))))
  (Development|PrintText (Utilities|Text|ToText(Boolean) _output_get)))