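; Actor component that tracks its owner's mental health, which drains in darkness and recovers out of it.
; Health starts at the clamped maximum with InDark set to true.
; While unpaused, a Delay on Tick throttles updates to about twice a second, each applying a clamped loss or faster gain, then firing OnChangeMentalHealth.
; TogglePause flips the pause flag that gates these updates.
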(event EventBeginPlay
  (Variables|Default|SetMentalHealth (Math|Float|Clamp(Float) (Variables|Default|GetMaxMentalHealth) 0.0 1e+02))
  (Variables|Default|SetInDark true))

(event EventTick
  (params (DeltaSeconds :type Float%20%28single-precision%29))
  (if (not (Variables|Default|GetIsPaused))
    (Utilities|FlowControl|Delay 0.5)
    (if (Variables|Default|GetInDark)
      (CallFunction|LoseMentalHealth 5.0)
      (else
        (CallFunction|GainMentalHealth 2e+01)))
    (Default|CallOnChangeMentalHealth)))

(fn LoseMentalHealth
  (params (value :type Float%20%28double-precision%29))
  (bind _output_get (Variables|Default|SetMentalHealth (Math|Float|Clamp(Float) (- (Variables|Default|GetMentalHealth) value) 0.0 (Variables|Default|GetMaxMentalHealth)))))

(fn GainMentalHealth
  (params (value :type Float%20%28double-precision%29))
  (bind _output_get (Variables|Default|SetMentalHealth (Math|Float|Clamp(Float) (+ (Variables|Default|GetMentalHealth) value) 0.0 (Variables|Default|GetMaxMentalHealth)))))

(fn TogglePause
  (bind _output_get (Variables|Default|SetIsPaused (not (Variables|Default|GetIsPaused)))))