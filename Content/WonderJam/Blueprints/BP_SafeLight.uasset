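; BP_SafeLight is a spot light actor with a capsule trigger, apparently meant as a lit safe zone for the player.
; The construction script sizes and offsets the capsule from the light's outer cone angle and attenuation radius, roughly approximating the lit volume.
; Overlap events only print debug text: entry is filtered to BP_FirstPersonCharacter, while exit fires for any actor.
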(event Collision|EventActorBeginOverlap
  (params (OtherActor :type Actor%20Object%20Reference))
  (Utilities|Casting|CastToBP_FirstPersonCharacter OtherActor)
  (Development|PrintText "ENTREE"))

(event Collision|EventActorEndOverlap
  (params (OtherActor :type Actor%20Object%20Reference))
  (Development|PrintText "SORTIE"))

(fn ConstructionScript
  (bind _spotlightcomponent (Variables|Default|GetSpotLightComponent))
  (bind _attenuationradius (Variables|/Script/Engine.LocalLightComponent|GetAttenuationRadius _spotlightcomponent))
  (Components|Capsule|SetCapsuleRadius (Variables|Default|GetCapsuleCollision) (* (Math|Trig|Tan(Degrees) (/ (Variables|/Script/Engine.SpotLightComponent|GetOuterConeAngle _spotlightcomponent) 2.0)) _attenuationradius) true)
  (Transformation|SetRelativeLocation (Variables|Default|GetCapsuleCollision) (Math|Vector|MakeVector _attenuationradius 0.0 0.0) false false)
  (Components|Capsule|SetCapsuleHalfHeight (Variables|Default|GetCapsuleCollision) _attenuationradius true))