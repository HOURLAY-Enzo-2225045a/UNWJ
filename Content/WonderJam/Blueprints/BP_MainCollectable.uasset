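; BP_MainCollectable is an interactable pickup that switches the player from the first-person character to a 2D character.
; Overlap registers it as the character's InteractObj and shows a HUD prompt, both cleared on exit.
; Interact updates the HUD collect count, destroys itself, then spawns and possesses a BP_CHAR2D at a fixed location, passing it a self-reference.
; It then spawns one BP_Spawner at that character per collected item.
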(event EventBeginPlay)

(event Collision|EventActorBeginOverlap
  (params (OtherActor :type Actor%20Object%20Reference))
  (Development|PrintText "Begin Overlap")
  (bind _asbp_first_person_character (Utilities|Casting|CastToBP_FirstPersonCharacter OtherActor)
    (:then
      (bind _output_get (Variables|Default|SetCharacter _asbp_first_person_character))
      (Variables|/Game/FirstPerson/Blueprints/BP_FirstPersonCharacter.BP_FirstPersonCharacter_C|SetInteractObj _output_get self)
      (bind _asbp_hud (Utilities|Casting|CastToBP_HUD (HUD|GetHUD (Game|GetPlayerController 0)))
        (:then
          (Variables|/Script/UMG.TextBlock|SetText (Variables|/Game/WonderJam/UI/UI_HUDDisplay.UI_HUDDisplay_C|GetInteractionText (Variables|/Game/WonderJam/Blueprints/BP_HUD.BP_HUD_C|GetUIReference _asbp_hud)) "Press [E] to interact"))
        (:CastFailed
          (Development|PrintText "Cast to HUD fail"))))
    (:CastFailed
      (Development|PrintText "Cast Failed"))))

(event Collision|EventActorEndOverlap
  (params (OtherActor :type Actor%20Object%20Reference))
  (bind _asbp_first_person_character (Utilities|Casting|CastToBP_FirstPersonCharacter OtherActor))
  (bind _output_get (Variables|Default|SetCharacter _asbp_first_person_character))
  (Variables|/Game/FirstPerson/Blueprints/BP_FirstPersonCharacter.BP_FirstPersonCharacter_C|SetInteractObj _output_get 0)
  (bind _asbp_hud (Utilities|Casting|CastToBP_HUD (HUD|GetHUD (Game|GetPlayerController 0))))
  (Variables|/Script/UMG.TextBlock|SetText (Variables|/Game/WonderJam/UI/UI_HUDDisplay.UI_HUDDisplay_C|GetInteractionText (Variables|/Game/WonderJam/Blueprints/BP_HUD.BP_HUD_C|GetUIReference _asbp_hud)) ""))

(event EventInteract
  (params (Controller :type Player%20Controller%20Object%20Reference))
  (bind _asbp_hud (Utilities|Casting|CastToBP_HUD (HUD|GetHUD Controller)))
  (Default|GetMoreCollect _asbp_hud)
  (Actor|DestroyActor)
  (bind _returnvalue (Game|SpawnActorfromClass "/Game/WonderJam/2D/BP_CHAR2D.BP_CHAR2D_C" (Math|Transform|MakeTransform "-80.000000,-60.000000,92.000000" "0, 0, 0" "1.000000,1.000000,1.000000") "Undefined" "MultiplyWithRoot" 0 0))
  (bind _output_get (Variables|Default|SetChar2D _returnvalue))
  (Variables|/Game/WonderJam/2D/BP_CHAR2D.BP_CHAR2D_C|SetMainCollectable _output_get self)
  (Pawn|Possess (Game|GetPlayerController 0) _output_get)
  (for _index (range 1 (Variables|/Game/WonderJam/Blueprints/BP_HUD.BP_HUD_C|GetCollectNum _asbp_hud))
    (Game|SpawnActorfromClass "/Game/WonderJam/2D/BP_Spawner.BP_Spawner_C" (Math|Conversions|ToTransform(Vector) (Transformation|GetActorLocation _output_get)) "Undefined" "MultiplyWithRoot" 0 0)))

(event EventOnFeedback)

(fn ConstructionScript)