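; BP_ProjectilePawn is a projectile for a 2D game that crosses the play area once over a few seconds, then destroys itself.
; On BeginPlay a random coin flip picks either a diagonal path to its XY-mirrored position or an axis-aligned path.
; The axis-aligned target comes from exact comparisons of spawn position against hard-coded arena edges, with positive Y as fallback.
; Overlapping BP_CHAR2D also destroys the projectile, with no damage applied here.
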(event EventBeginPlay
  (bind _returnvalue (Transformation|GetActorLocation))
  (bind _returnvalue_2 (Transformation|GetActorLocation))
  (bind _rootcomponent (Variables|Transformation|GetRootComponent))
  (bind _result (CallFunction|Randomise))
  (if _result
    (Components|MoveComponentTo (Variables|Transformation|GetRootComponent) (* (Transformation|GetActorLocation) "-1.000000,-1.000000,1.000000") "0, 0, 0" false false 3.0 false)
    (else
      (Math|Float|CompareFloat (.x _returnvalue_2) 4e+02
        (:>
          (Math|Float|CompareFloat (.y _returnvalue_2) 8.5e+02 :!label _label
            (:>
              (Math|Float|CompareFloat (.y _returnvalue_2) -8.5e+02 :!label _label_2
                (:>
                  _)
                (:==
                  _)
                (:<
                  _))
              (Components|MoveComponentTo _rootcomponent (Math|Vector|MakeVector (.x _returnvalue) 8.5e+02 (.z _returnvalue)) "0, 0, 0" false false 3.0 false))
            (:==
              (Components|MoveComponentTo _rootcomponent (Math|Vector|MakeVector (.x _returnvalue) -8.5e+02 (.z _returnvalue)) "0, 0, 0" false false 3.0 false))
            (:<
              (goto _label_2))))
        (:==
          (Components|MoveComponentTo _rootcomponent (Math|Vector|MakeVector -5.3e+02 (.y _returnvalue) (.z _returnvalue)) "0, 0, 0" false false 3.0 false))
        (:<
          (Math|Float|CompareFloat (.x _returnvalue_2) -5.3e+02
            (:>
              (goto _label))
            (:==
              (Components|MoveComponentTo _rootcomponent (Math|Vector|MakeVector 4e+02 (.y _returnvalue) (.z _returnvalue)) "0, 0, 0" false false 3.0 false))
            (:<
              (goto _label)))))))
  (Actor|DestroyActor))

(event Collision|EventActorBeginOverlap
  (params (OtherActor :type Actor%20Object%20Reference))
  (Utilities|Casting|CastToBP_CHAR2D OtherActor)
  (Actor|DestroyActor))

(fn ConstructionScript)

(fn Randomise
  (Math|Float|CompareFloat (Math|Random|RandomFloatinRange -1.0 1.0) 0.0
    (:>
      _)
    (:==
      _)
    (:<
      (return false)))
  (return true))