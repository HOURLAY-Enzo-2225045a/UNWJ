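; BP_Spawner spawns a short timed series of BP_ProjectilePawn actors when play begins.
; BeginPlay drives a custom loopWithDelay macro, a for-loop that waits between iterations, to spawn six pawns a second apart.
; Each pawn appears at a random X and Y within hardcoded bounds at a fixed height, independent of the spawner's own location.
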(event EventBeginPlay
  (Utilities|LoopwithDelay 0 5 1.0
    (:loop%20Body
      (Game|SpawnActorfromClass "/Game/WonderJam/2D/BP_ProjectilePawn.BP_ProjectilePawn_C" (Math|Transform|MakeTransform (Math|Vector|MakeVector (Math|Random|RandomFloatinRange -5.3e+02 4e+02) (Math|Random|RandomFloatinRange -8.5e+02 8.5e+02) 92.0) "0, 0, 0" "1.000000,1.000000,1.000000") "Undefined" "MultiplyWithRoot" 0 0))))

(fn ConstructionScript)